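; Interactable object that highlights with an outline mesh while being looked at and supplies its name and details.
; Seen shows the outline, which starts hidden, and returns Name and Details to the caller.
; A short retriggerable delay hides the outline once Seen stops being called, so no explicit unfocus call is needed.
; Interaction is a placeholder that only prints a message saying it can't do anything.
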(event `self.ReceiveBeginPlay`
  (`SceneComponent.SetVisibility` (`self.outline mesh`) false false))

(event `/Game/_Interactions/11-Interaction.Interaction`
  (`KismetSystemLibrary.PrintString` "Hello, I can't do anything!"))

(event `Turn On Outline`
  (`SceneComponent.SetVisibility` (`self.outline mesh`) true false)
  (`self.Timer to forget`))

(event `Timer to forget`
  (`KismetSystemLibrary.RetriggerableDelay` 0.2)
  (`SceneComponent.SetVisibility` (`self.outline mesh`) false false))

(fn `Seen`
  (returns (Details :type Text) (Name :type Text))
  (`self.Turn On Outline`)
  (return (`self.Details`) (`self.Name`)))

(fn `UserConstructionScript`)